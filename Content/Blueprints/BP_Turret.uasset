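; Turret actor that uses PawnSensing to detect the BP_FPCharacter player and snaps its whole body to face them on each sighting.
; After a RateOfFire delay it spawns an actor at the Scene component, then after 2ndRateOfFire another at Scene1.
; The Delays pace firing, since repeated sightings do not restart them.
; FindBestTarget and the construction script are empty.
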(event OnSeePawn(PawnSensing)
  (params (Pawn :type Pawn%20Object%20Reference))
  (Utilities|Casting|CastToBP_FPCharacter Pawn)
  (Transformation|SetActorRotation (Math|Rotator|FindLookatRotation (Transformation|GetActorLocation) (Transformation|GetActorLocation Pawn)))
  (Utilities|FlowControl|Delay (Variables|Default|GetRate%20of%20fire))
  (Game|SpawnActorfromClass "/Game/Blueprints/BP_Projectile.BP_Projectile_C" (Transformation|GetSocketTransform (Variables|Default|GetScene) "None" "RTS_World") "Undefined" "MultiplyWithRoot" 0 0)
  (Utilities|FlowControl|Delay (Variables|Default|Get2nd%20rate%20of%20fire))
  (Game|SpawnActorfromClass "/Game/Blueprints/BP_Projectile.BP_Projectile_C" (Transformation|GetSocketTransform (Variables|Default|GetScene1) "None" "RTS_World") "Undefined" "MultiplyWithRoot" 0 0))

(event Collision|EventActorBeginOverlap
  (params (OtherActor :type Actor%20Object%20Reference)))

(fn ConstructionScript)

(fn FindBestTarget)