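; BP_Enemy is an enemy character that runs toward the objective actor in the level.
; On BeginPlay it starts a looping run animation and audio, then sets walk speed, takes the first BP_Objective found as its target and issues an AI MoveTo.
; Tick re-enters that same chain, so the speed setting, all-actors search and move request repeat every frame.
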(event EventBeginPlay
  (Components|Animation|PlayAnimation (Variables|Character|GetMesh) "/Game/Blueprints/Player/Running_mixamo_com.Running_mixamo_com" true)
  (Audio|Components|Audio|Play (Variables|Default|GetAudio) 0.0)
  (Variables|/Script/Engine.CharacterMovementComponent|SetMaxWalkSpeed (Variables|Character|GetCharacterMovement) 4e+02)
  (CallFunction|Locate)
  (AI|AIMoveTo self "0, 0, 0" (Variables|Default|GetObjective) 1.0 false))

(event Collision|EventActorBeginOverlap
  (params (OtherActor :type Actor%20Object%20Reference)))

(event EventTick
  (params (DeltaSeconds :type Float%20%28single-precision%29))
  (Variables|/Script/Engine.CharacterMovementComponent|SetMaxWalkSpeed (Variables|Character|GetCharacterMovement) 4e+02)
  (CallFunction|Locate)
  (AI|AIMoveTo self "0, 0, 0" (Variables|Default|GetObjective) 1.0 false))

(fn ConstructionScript)

(fn Locate
  (bind _outactors (Actor|GetAllActorsOfClass "/Game/Blueprints/BP_Objective.BP_Objective_C"))
  (Variables|Default|SetObjective (Utilities|Array|Get(acopy) _outactors)))

(fn Blueppoit)